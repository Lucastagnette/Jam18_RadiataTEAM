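; BP_Test is a test Blueprint that pushes a Cube component forward, resembling a stripped-down flying movement controller.
; Tick moves the cube along local X at ForwardSpeed, scaled by delta time, with sweep collision.
; The TurnRight axis eases CurrentYawSpeed toward input times RightRotation via FInterpTo, but nothing applies that value as rotation.
; An unconnected FInterpTo chain holds roll-based yaw logic that never runs.
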(event EventTick
  (params (DeltaSeconds :type Float%20%28single-precision%29))
  ;[0 0 0] Go Forward
  (Transformation|AddLocalOffset (Variables|Default|GetCube) (Math|Vector|MakeVector (* DeltaSeconds (Variables|Default|GetForwardSpeed)) 0.0 0.0) true false))

(event Input|AxisEvents|InputAxisTurnRight
  (params (AxisValue :type Float%20%28single-precision%29))
  (Variables|Default|SetCurrentYawSpeed (Math|Interpolation|FInterpTo (Variables|Default|GetCurrentYawSpeed) (* AxisValue (Variables|Default|GetRight%20Rotation)) (Utilities|Time|GetWorldDeltaSeconds) 2.0)))

(fn ConstructionScript)