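; BP_Submarine is the player submarine, which constantly moves forward and steers by yaw input.
; A timed loop cycles through forced effects: a speed dash, an instant 180-degree turn and temporarily inverted steering.
; Damage reduces life with screen, sound and shake feedback, ending in destruction and a death UI, while DestroyerSphere overlaps destroy bullets and enemies and count kills.
; BeginPlay also sets the CameraManager view, engine sound and life HUD.
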(event OnComponentBeginOverlap(destroyerSphere)
  (params (OverlappedComponent :type Primitive%20Component%20Object%20Reference) (OtherActor :type Actor%20Object%20Reference) (OtherComp :type Primitive%20Component%20Object%20Reference) (OtherBodyIndex :type Integer) (bFromSweep :type Boolean) (SweepResult :type Hit%20Result%20Structure%20%28by%20ref%29))
  ;[0.1356 0.01096 0.02122] PrrojectileDestruction
  (Utilities|FlowControl|Sequence
    (:then_0
      (bind _asbullets (Utilities|Casting|CastToBullets OtherActor))
      (Actor|DestroyActor _asbullets)
      (Variables|Default|SetEnnemies_Killed (+ (Variables|Default|GetEnnemies_Killed) 1))
      (Audio|PlaySound2D "/Game/SFX/hitEnemy.hitEnemy" 1.0 1.0 0.0 0 0))
    (:then_1
      (bind _asennemi (Utilities|Casting|CastToEnnemi OtherActor))
      (Actor|DestroyActor _asennemi)
      (Variables|Default|SetEnnemies_Killed (+ (Variables|Default|GetEnnemies_Killed) 1))
      (Audio|PlaySound2D "/Game/SFX/hitEnemy.hitEnemy" 1.0 1.0 0.0 0 0))))

(event EventBeginPlay
  (bind _returnvalue (Game|GetPlayerController 0))
  (Utilities|FlowControl|Sequence
    (:then_0
      (Input|DisableInput _returnvalue)
      (Utilities|FlowControl|Delay 1.0)
      (Input|EnableInput _returnvalue))
    (:then_1
      ;[1 0.8912 0] Camera Change
      (bind _returnvalue_2 (Actor|GetActorOfClass "/Game/CharacterBP/CameraManager.CameraManager_C"))
      (Game|Player|SetViewTargetwithBlend (Game|GetPlayerController 0) _returnvalue_2 0.0 "VTBlend_Linear" 0.0 false))
    (:then_2
      ;[0 0.61 1] Capacity Loop
      (Utilities|FlowControl|Delay 1e+01 :!label _label)
      (switch int (Variables|Default|GetCapacityOrder)
        (:0
          (Variables|Default|SetCapacityOrder (+ (Variables|Default|GetCapacityOrder) 1))
          (Utilities|Dash)
          (Development|PrintString "1")
          (goto _label))
        (:1
          (Variables|Default|SetCapacityOrder (+ (Variables|Default|GetCapacityOrder) 1))
          (Utilities|180)
          (Development|PrintString "2")
          (goto _label))
        (:2
          (Variables|Default|SetNewVar_1 -1)
          (Utilities|FlowControl|Delay 1e+01)
          (Variables|Default|SetNewVar_1 1)
          (Variables|Default|SetCapacityOrder 0)
          (Development|PrintString "3" true true "(R=1.000000,G=0.000000,B=0.080943,A=1.000000)")
          (goto _label))))
    (:then_3
      (bind _returnvalue_3 (Audio|SpawnSound2D "/Game/SFX/Boat.Boat" 1.0 1.0 0.0 0))
      (Variables|Default|SetSoundBoat _returnvalue_3))
    (:then_4
      (bind _returnvalue_4 (UserInterface|CreateWidget "/Game/UI-UX/UI/LifeInGame.LifeInGame_C"))
      (UserInterface|Viewport|AddtoViewport _returnvalue_4 0))))

(event EventTick
  (params (DeltaSeconds :type Float%20%28single-precision%29))
  (bind _returnvalue (Transformation|GetActorForwardVector))
  ;[0.04231 0.4072 0] Movements
  (Utilities|FlowControl|Sequence
    (:then_1
      (Variables|/Script/Engine.MovementComponent|SetVelocity (Variables|Default|GetMovementComponent) (* _returnvalue (+ _returnvalue (Variables|Default|GetForward_Force)))))
    (:then_2
      ;[1 0.3769 0.9147] Timer
      (Utilities|FlowControl|Delay 1.0)
      (Variables|Default|SetSecond%20 (+ (Variables|Default|GetSecond%20) 1)))))

(event Game|Damage|EventAnyDamage
  (params (Damage :type Float%20%28single-precision%29) (DamageType :type Damage%20Type%20Object%20Reference) (InstigatedBy :type Controller%20Object%20Reference) (DamageCauser :type Actor%20Object%20Reference))
  ;[1 0 0.02464] Life Damages
  (Variables|Default|SetLife (- (Variables|Default|GetLife) Damage))
  (bind _returnvalue (UserInterface|CreateWidget "/Game/UI-UX/UI/DamagesScreen.DamagesScreen_C"))
  (UserInterface|Viewport|AddtoViewport _returnvalue 0)
  (Audio|PlaySound2D "/Game/SFX/BrokenClass.BrokenClass" 1.0 1.0 0.0 0 0)
  (Camera|PlayWorldCameraShake "/Script/Engine.CameraShakeBase" "0, 0, 0" 0.0 0.0)
  (if (<= (Variables|Default|GetLife) 0.0)
    (Audio|Components|Audio|Stop (Variables|Default|GetSoundBoat))
    (Actor|DestroyActor)
    (bind _returnvalue_2 (UserInterface|CreateWidget "/Game/UI-UX/UI/DeathUI.DeathUI_C"))
    (UserInterface|Viewport|AddtoViewport _returnvalue_2 0)
    (else
      (Default|TEST (stale EventBeginPlay _returnvalue_4)))))

(event Input|AxisEvents|InputAxisTurnRight
  (params (AxisValue :type Float%20%28single-precision%29))
  ;[0.1039 1 0] Rotation
  (Transformation|AddActorLocalRotation (Math|Rotator|MakeRotator 0.0 0.0 (* AxisValue 2.0 (Variables|Default|GetNewVar_1))) false false))

(fn ConstructionScript)